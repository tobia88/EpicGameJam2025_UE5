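; BP_PlatformController fills a box area with a grid of child platform actors of a configurable class.
; RefreshPlatforms clears existing child components, then derives rounded X and Y counts, at least one each, from box extent and platform size.
; SpawnPlatfom offsets each cell by half the grid bounds and converts it through the box transform into actor-relative space.
; Construction script and events are empty, so nothing here calls the refresh.
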(event EventBeginPlay)

(event Collision|EventActorBeginOverlap
  (params (OtherActor :type Actor%20Object%20Reference)))

(event EventTick
  (params (DeltaSeconds :type Float%20%28single-precision%29)))

(fn ConstructionScript)

(fn RefreshPlatforms
  (bind _box (Variables|Default|GetBox))
  (bind _platformsize (Variables|Default|GetPlatformSize))
  (bind _returnvalue (Components|Box|GetScaledBoxExtent _box))
  (bind _returnvalue_2 (* _returnvalue 2.0))
  (bind _returnvalue_3 (/ (Math|Vector2D|MakeVector2D (.x _returnvalue_2) (.y _returnvalue_2)) _platformsize))
  (bind (_x _y) (Math|Vector2D|BreakVector2D _returnvalue_3))
  (CallFunction|ClearChildActors)
  (bind _output_get (Variables|Default|SetXLength (Math|Integer|Max(Integer) (Math|Float|Round _x) 1)))
  (bind _output_get_2 (Variables|Default|SetYLength (Math|Integer|Max(Integer) (Math|Float|Round _y) 1)))
  (Variables|Default|SetBoundSize (* (Math|Vector2D|MakeVector2D (Math|Conversions|ToFloat(Integer) _output_get) (Math|Conversions|ToFloat(Integer) _output_get_2)) (Variables|Default|GetPlatformSize)))
  (for _index (range 0 (- (Variables|Default|GetYLength) 1))
    (for _index_2 (range 0 (- (Variables|Default|GetXLength) 1))
      (CallFunction|SpawnPlatfom _index_2 _index))))

(fn SpawnPlatfom
  (params (x :type Integer) (y :type Integer))
  (bind _returnvalue (Transformation|GetActorTransform))
  (bind _box (Variables|Default|GetBox))
  (bind _platformsize (Variables|Default|GetPlatformSize))
  (bind _boundsize (Variables|Default|GetBoundSize))
  (bind _returnvalue_2 (Math|Transform|InvertTransform _returnvalue))
  (bind _returnvalue_3 (Transformation|GetWorldTransform _box))
  (bind _returnvalue_4 (* x (.x _platformsize)))
  (bind _returnvalue_5 (* y (.y _platformsize)))
  (bind _returnvalue_6 (* _boundsize 0.5))
  (bind _returnvalue_7 (Math|Transform|ComposeTransforms _returnvalue_3 _returnvalue_2))
  (bind _returnvalue_8 (Math|Vector2D|MakeVector2D _returnvalue_4 _returnvalue_5))
  (bind _returnvalue_9 (- _returnvalue_8 _returnvalue_6))
  (bind _returnvalue_10 (Math|Transform|MakeTransform (Math|Vector|MakeVector (.x _returnvalue_9) (.y _returnvalue_9) 0.0)))
  (bind _returnvalue_11 (Math|Transform|ComposeTransforms _returnvalue_10 _returnvalue_7))
  (bind _returnvalue_12 (AddComponent|AddChildActorComponent false (Math|Transform|MakeTransform (.location _returnvalue_11) (.rotation _returnvalue_11) "1.000000,1.000000,1.000000")))
  (Utilities|Array|Add (Variables|Default|GetChildActors) _returnvalue_12)
  (ChildActorComponent|SetChildActorClass _returnvalue_12 (Variables|Default|GetPlatformActorClass)))

(fn ClearChildActors
  (bind _arrayelement (Utilities|Array|ReverseforEachLoop 0)
    (:LoopBody
      (Utilities|IsValid _arrayelement
        (:Is%20Valid
          (Components|DestroyComponent _arrayelement))))
    (:Completed
      (Utilities|Array|Clear (Variables|Default|GetChildActors)))))