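; BP_EMJEnemyCharacter is an enemy character with simple hit points that is destroyed when its health runs out.
; On BeginPlay it copies BaseHP into CurrentHP; the Damage event subtracts through SetHp, then destroys the actor if GetShouldDead finds HP at or below zero.
; DoAttack is an empty event, and a projectile spawn node sits unconnected.
; EvaluateShouldDead duplicates GetShouldDead and is not called here.
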(event EventBeginPlay
  (CallFunction|InitAttributes))

(event Collision|EventActorBeginOverlap
  (params (OtherActor :type Actor%20Object%20Reference)))

(event EventTick
  (params (DeltaSeconds :type Float%20%28single-precision%29)))

(event EventDoAttack)

(event EventDamage
  (params (Damage :type Float%20%28double-precision%29))
  (CallFunction|SetHp (- (Variables|Default|GetCurrentHP) Damage))
  (if (CallFunction|GetShouldDead)
    (Actor|DestroyActor)))

(fn ConstructionScript)

(fn InitAttributes
  (Variables|Default|SetCurrentHP (Variables|Default|GetBaseHP)))

(fn SetHp
  (params (NewHp :type Float%20%28double-precision%29))
  (Variables|Default|SetCurrentHP NewHp))

(fn GetShouldDead
  (return (<= (Variables|Default|GetCurrentHP) 0.0)))

(fn EvaluateShouldDead
  (return (<= (Variables|Default|GetCurrentHP) 0.0)))