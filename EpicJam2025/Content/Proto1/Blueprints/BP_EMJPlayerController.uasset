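; BP_EMJPlayerController is a player controller that sets up Enhanced Input and samples movement and look input.
; On BeginPlay, it adds the platforming and mouse-look mapping contexts for local players only.
; Each Tick polls the input action values, storing movement in MoveInput and the sum of mouse and regular look input in LookInput.
; The graph only stores these values and does not apply them to a pawn.
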(event EventBeginPlay
  (bind _returnvalue (PlayerController|LocalPlayerSubsystems|GetEnhancedInputLocalPlayerSubsystem))
  (if (Pawn|IsLocalPlayerController)
    (Input|AddMappingContext _returnvalue "/Game/Variant_Platforming/Input/IMC_Platforming.IMC_Platforming" 0 "(bIgnoreAllPressedKeysUntilRelease=True,bForceImmediately=False,bNotifyUserSettings=False)")
    (Input|AddMappingContext _returnvalue "/Game/Input/IMC_MouseLook.IMC_MouseLook" 0 "(bIgnoreAllPressedKeysUntilRelease=True,bForceImmediately=False,bNotifyUserSettings=False)")))

(event EventTick
  (params (DeltaSeconds :type Float%20%28single-precision%29))
  (Variables|Default|SetMoveInput (Input|EnhancedActionValues|GetIA_Move))
  (Variables|Default|SetLookInput (+ (Input|EnhancedActionValues|GetIA_MouseLook) (Input|EnhancedActionValues|GetIA_Look))))

(fn ConstructionScript)