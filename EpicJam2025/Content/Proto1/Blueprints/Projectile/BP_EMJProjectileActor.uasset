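; BP_EMJProjectileActor is a combat projectile that flies straight along its forward vector at MoveSpeed.
; Each tick it moves without sweeping, then sphere-traces from its previous to new location using CombatCollision's radius, ignoring its owner and drawing debug shapes.
; Any hits go to BP_EMJGameMode's CombatProcessProjectileHit with a blocking flag, so the game mode handles resolution.
; GetDamage exposes base damage scaled by DamageMultiplier.
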(event EventTick
  (params (DeltaSeconds :type Float%20%28single-precision%29))
  (Variables|Default|SetPrevLocation (Transformation|GetActorLocation))
  (bind _output_get (Variables|Default|SetVelocityThisFrame (* (Math|Vector|GetForwardVector (Transformation|GetActorRotation)) (* DeltaSeconds (Variables|Default|GetMoveSpeed)))))
  (Transformation|AddActorWorldOffset _output_get)
  (bind (_outhits _returnvalue) (Collision|MultiSphereTraceByChannel (Variables|Default|GetPrevLocation) (Transformation|GetActorLocation) (Components|Sphere|GetScaledSphereRadius (Variables|Default|GetCombatCollision)) "TraceTypeQuery3" false (Utilities|Array|MakeArray (Variables|Default|GetOwnerActor)) "ForDuration" true "(R=1.000000,G=0.000000,B=0.000000,A=1.000000)" "(R=0.000000,G=1.000000,B=0.000000,A=1.000000)" (Variables|Debug|GetDraw%20Time)))
  (if (Utilities|Array|IsNotEmpty _outhits)
    (CallFunction|OnHit _outhits _returnvalue)))

(fn ConstructionScript)

(fn OnHit
  (params (HitResults :type Array%20of%20Hit%20Result%20Structures) (bIsBlocking :type Boolean))
  (bind _asbp_emjgame_mode (Utilities|Casting|CastToBP_EMJGameMode (Game|GetGameMode)))
  (Default|CombatProcessProjectileHit _asbp_emjgame_mode self HitResults bIsBlocking))

(fn GetDamage
  (return (* (Variables|Default|GetDamage) (Variables|Default|GetDamageMultiplier))))