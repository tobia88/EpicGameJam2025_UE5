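; BP_EMJGameMode is a prototype game mode Blueprint that centrally resolves projectile hits for combat.
; CombatProcessProjectileHit sends the projectile's Damage to each hit actor with a debug print, then notifies the projectile's valid owner through OnProjectileHitMessage.
; It destroys the projectile afterward only when the hit is flagged as blocking.
; OnPowerCordHit is a stub that loops over hit results without acting, and the event graph is unused.
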(event EventBeginPlay)

(event EventTick
  (params (DeltaSeconds :type Float%20%28single-precision%29)))

(fn ConstructionScript)

(fn OnPowerCordHit
  (params (Power%20Cord%20Actor :type BP%20Power%20Cord%20Projectile%20Object%20Reference) (Hit%20Results :type Array%20of%20Hit%20Result%20Structures))
  (for _array_element Hit%20Results
    _))

(fn CombatProcessProjectileHit
  (params (ProjectileActor :type BP%20EMJ%20Projectile%20Actor%20Object%20Reference) (HitResults :type Array%20of%20Hit%20Result%20Structures) (bIsBlockHit :type Boolean))
  (CallFunction|CombatProcessDamage ProjectileActor HitResults)
  (CallFunction|CombatProcessBroadcastEvents ProjectileActor HitResults)
  (if bIsBlockHit
    (Actor|DestroyActor ProjectileActor)))

(fn CombatProcessDamage
  (params (ProjectileActor :type BP%20EMJ%20Projectile%20Actor%20Object%20Reference) (HitResults :type Array%20of%20Hit%20Result%20Structures))
  (for _array_element HitResults
    (Class|BPICombatableActor|ReceiveDamage(Message) (.HitActor (Collision|BreakHitResult _array_element)) (Variables|/Game/Proto1/Blueprints/Projectile/BP_EMJProjectileActor.BP_EMJProjectileActor_C|GetDamage ProjectileActor))
    (Development|PrintString (Utilities|String|ToString(Text) (Utilities|Text|FormatText "GameMode: CombatProcessDamage: {projectile} Hit {actor}" ProjectileActor (.HitActor (Collision|BreakHitResult _array_element)))))))

(fn CombatProcessBroadcastEvents
  (params (ProjectileActor :type BP%20EMJ%20Projectile%20Actor%20Object%20Reference) (HitResults :type Array%20of%20Hit%20Result%20Structures))
  (bind _owneractor (Variables|/Game/Proto1/Blueprints/Projectile/BP_EMJProjectileActor.BP_EMJProjectileActor_C|GetOwnerActor ProjectileActor)
    (:then
      (Class|BPICombatableActor|OnProjectileHit(Message) _owneractor ProjectileActor HitResults))
    (:else)))