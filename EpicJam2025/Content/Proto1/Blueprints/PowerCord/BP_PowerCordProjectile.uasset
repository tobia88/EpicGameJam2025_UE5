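; BP_PowerCordProjectile is the moving projectile for the player's power cord, detecting what the cord hits.
; Each Tick moves it forward by MoveSpeed without sweeping, then sphere-traces from the previous location to the new one using the CombatCollision radius on the Visibility channel.
; The trace ignores OwnerPlayer, draws debug shapes and passes any hits to OwnerPlayer.OnCordHitActor.
; The projectile never stops or destroys itself here.
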(event EventBeginPlay)

(event Collision|EventActorBeginOverlap
  (params (OtherActor :type Actor%20Object%20Reference)))

(event EventTick
  (params (DeltaSeconds :type Float%20%28single-precision%29))
  (Variables|Default|SetPrevLocation (Transformation|GetActorLocation))
  (bind _output_get (Variables|Default|SetVelocityThisFrame (* (Math|Vector|GetForwardVector (Transformation|GetActorRotation)) (* DeltaSeconds (Variables|Default|GetMoveSpeed)))))
  (Transformation|AddActorWorldOffset _output_get)
  (bind _outhits (Collision|MultiSphereTraceByChannel (Variables|Default|GetPrevLocation) (Transformation|GetActorLocation) (Components|Sphere|GetScaledSphereRadius (Variables|Default|GetCombatCollision)) "TraceTypeQuery1" false (Utilities|Array|MakeArray (Variables|Default|GetOwnerPlayer)) "ForDuration"))
  (if (Utilities|Array|IsNotEmpty _outhits)
    (Default|OnCordHitActor (Variables|Default|GetOwnerPlayer) _outhits)))

(fn ConstructionScript)