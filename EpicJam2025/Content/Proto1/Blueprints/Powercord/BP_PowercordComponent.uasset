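; Player character component for a power cord that tethers the owner to a target actor.
; Setting the target binds it to the capsule through the owner's physics constraint, or clears the constraint.
; DoTick shows and stretches a supplied spline mesh from the spine socket to the target.
; ClampOwnerMovement iteratively steps an over-length position toward the target using debug-drawn downward sphere traces within step height, then forces corrective movement input.
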(event EventBeginPlay)

(event EventTick
  (params (DeltaSeconds :type Float%20%28single-precision%29)))

(fn Init)

(fn DoTick
  (params (DeltaTime :type Float%20%28double-precision%29))
  (CallFunction|TickRender))

(fn SetMesh
  (params (SplineMeshComponent :type Spline%20Mesh%20Component%20Object%20Reference))
  (Variables|Default|SetSplineMeshComponent SplineMeshComponent))

(fn TickRender
  (bind _splinemeshcomponent (Variables|Default|GetSplineMeshComponent))
  (CallFunction|RefreshSplineMeshVisibility)
  (Variables|Default|GetTargetAttachActor
    (:then
      (Rendering|Material|SetCustomPrimitiveDataFloat (Variables|Default|GetSplineMeshComponent) 0 (Math|Conversions|ToFloat(Boolean) (CallFunction|GetIsAttaching)))
      (SplineMesh|SetStartPosition _splinemeshcomponent (Transformation|GetSocketLocation (Variables|/Script/Engine.Character|GetMesh (CallFunction|GetOwnerCharacter)) "spine_03") false)
      (SplineMesh|SetEndPosition _splinemeshcomponent (Transformation|GetActorLocation (Variables|Default|GetTargetAttachActor)) false)
      (SplineMesh|UpdateMesh _splinemeshcomponent))
    (:else)))

(fn GetOwnerCharacter
  (return (.AsBP%20EMJPlayer%20Character (Utilities|Casting|CastToBP_EMJPlayerCharacter (Components|GetOwner)))))

(fn SetTargetAttachActor
  (params (TargetAttachActor :type Actor%20Object%20Reference))
  (bind _asbp_emjplayer_character (CallFunction|GetOwnerCharacter))
  (bind _physicsconstraint (Variables|/Game/Proto1/Blueprints/BP_EMJPlayerCharacter.BP_EMJPlayerCharacter_C|GetPhysicsConstraint _asbp_emjplayer_character))
  (bind _output_get (Variables|Default|SetTargetAttachActor TargetAttachActor))
  (Utilities|IsValid _output_get
    (:Is%20Valid
      (Class|PhysicsConstraintComponent|SetConstrainedComponents _physicsconstraint (Actor|GetComponentbyClass _output_get "/Script/Engine.PrimitiveComponent") "None" (Variables|/Script/Engine.Character|GetCapsuleComponent _asbp_emjplayer_character) "None"))
    (:Is%20Not%20Valid
      (Class|PhysicsConstraintComponent|SetConstrainedComponents _physicsconstraint 0 "None" 0 "None"))))

(fn GetIsAttaching
  (return (Utilities|IsValid (Variables|Default|GetTargetAttachActor))))

(fn RefreshSplineMeshVisibility
  (Rendering|SetVisibility (Variables|Default|GetSplineMeshComponent) (Utilities|IsValid (Variables|Default|GetTargetAttachActor)) false))

(fn GetCordLength
  (bind _targetattachactor (Variables|Default|GetTargetAttachActor)
    (:then
      (return (Transformation|GetDistanceTo _targetattachactor (Components|GetOwner))))
    (:else
      (return 0.0))))

(fn ClampOwnerMovement
  (bind _asbp_emjplayer_character (CallFunction|GetOwnerCharacter))
  (bind _asbp_emjplayer_character_2 (CallFunction|GetOwnerCharacter))
  (bind _asbp_emjplayer_character_3 (CallFunction|GetOwnerCharacter))
  (bind _returnvalue (Transformation|GetActorLocation _asbp_emjplayer_character_2))
  (bind _returnvalue_2 (Class|Pawn|GetPendingMovementInputVector _asbp_emjplayer_character_2))
  (bind _charactermovement (Variables|/Script/Engine.Character|GetCharacterMovement _asbp_emjplayer_character_3))
  (bind _capsulecomponent (Variables|/Script/Engine.Character|GetCapsuleComponent _asbp_emjplayer_character))
  (bind _returnvalue_3 (Components|Capsule|GetScaledCapsuleHalfHeight _capsulecomponent))
  (bind _returnvalue_4 (+ _returnvalue _returnvalue_2))
  (bind _maxstepheight (Variables|/Script/Engine.CharacterMovementComponent|GetMaxStepHeight _charactermovement))
  (if (CallFunction|GetIsAttaching)
    (LocalVariables|SetStartLoc _returnvalue_4)
    (LocalVariables|SetDesiredLoc _returnvalue_4)
    (Utilities|FlowControl|ForLoopwithBreak 0 5 :!label _label
      (:LoopBody
        (if (> (Math|Vector|VectorLength (- (Transformation|GetActorLocation (Variables|Default|GetTargetAttachActor)) (LocalVariables|GetDesiredLoc))) (Variables|Default|GetMaxCordLength))
          (bind (_outhit _returnvalue_5) (Collision|SphereTraceByChannel (+ (LocalVariables|GetDesiredLoc) (* (Math|Vector|SelectVector (Transformation|GetActorForwardVector (CallFunction|GetOwnerCharacter)) (/ (- (Transformation|GetActorLocation (Variables|Default|GetTargetAttachActor)) (LocalVariables|GetDesiredLoc)) (Math|Vector|VectorLength (- (Transformation|GetActorLocation (Variables|Default|GetTargetAttachActor)) (LocalVariables|GetDesiredLoc)))) (Math|Float|NearlyEqual(Float) (Math|Vector|VectorLength (- (Transformation|GetActorLocation (Variables|Default|GetTargetAttachActor)) (LocalVariables|GetDesiredLoc))) 0.0 1e-06)) 15.0)) (- (+ (LocalVariables|GetDesiredLoc) (* (Math|Vector|SelectVector (Transformation|GetActorForwardVector (CallFunction|GetOwnerCharacter)) (/ (- (Transformation|GetActorLocation (Variables|Default|GetTargetAttachActor)) (LocalVariables|GetDesiredLoc)) (Math|Vector|VectorLength (- (Transformation|GetActorLocation (Variables|Default|GetTargetAttachActor)) (LocalVariables|GetDesiredLoc)))) (Math|Float|NearlyEqual(Float) (Math|Vector|VectorLength (- (Transformation|GetActorLocation (Variables|Default|GetTargetAttachActor)) (LocalVariables|GetDesiredLoc))) 0.0 1e-06)) 15.0)) (Math|Vector|MakeVector 0.0 0.0 (+ _returnvalue_3 _maxstepheight 1e+01))) (Components|Capsule|GetScaledCapsuleRadius _capsulecomponent) "TraceTypeQuery1" false 0 "ForDuration"))
          (if _returnvalue_5
            (if (<= (- (.Z (Math|Vector|BreakVector (+ (.ImpactPoint (Collision|BreakHitResult _outhit)) (Math|Vector|MakeVector 0.0 0.0 _returnvalue_3)))) (.Z (Math|Vector|BreakVector (+ (LocalVariables|GetDesiredLoc) (* (Math|Vector|SelectVector (Transformation|GetActorForwardVector (CallFunction|GetOwnerCharacter)) (/ (- (Transformation|GetActorLocation (Variables|Default|GetTargetAttachActor)) (LocalVariables|GetDesiredLoc)) (Math|Vector|VectorLength (- (Transformation|GetActorLocation (Variables|Default|GetTargetAttachActor)) (LocalVariables|GetDesiredLoc)))) (Math|Float|NearlyEqual(Float) (Math|Vector|VectorLength (- (Transformation|GetActorLocation (Variables|Default|GetTargetAttachActor)) (LocalVariables|GetDesiredLoc))) 0.0 1e-06)) 15.0))))) _maxstepheight)
              (LocalVariables|SetDesiredLoc (+ (.ImpactPoint (Collision|BreakHitResult _outhit)) (Math|Vector|MakeVector 0.0 0.0 _returnvalue_3)))
              (else
                (goto _label Break)))
            (else
              (goto _label Break)))
          (else
            (goto _label Break))))
      (:Completed
        (if (not (Math|Float|NearlyEqual(Float) (Math|Vector|VectorLength (- (LocalVariables|GetDesiredLoc) (LocalVariables|GetStartLoc))) 0.0 1e-06))
          (Pawn|Input|AddMovementInput (CallFunction|GetOwnerCharacter) (/ (- (LocalVariables|GetDesiredLoc) (LocalVariables|GetStartLoc)) (Math|Vector|VectorLength (- (LocalVariables|GetDesiredLoc) (LocalVariables|GetStartLoc)))) (Math|Vector|VectorLength (- (LocalVariables|GetDesiredLoc) (LocalVariables|GetStartLoc))) true))))))